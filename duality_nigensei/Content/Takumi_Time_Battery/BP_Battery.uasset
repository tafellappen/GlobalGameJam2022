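; BP_Battery is a pickup that adds ten seconds to the time limit when a TopDownCharacter overlaps its Box.
; It writes directly to the character's UITimeLimit widget, playing the PlusTime animation, carrying overflow seconds into minutes and refreshing the text.
; Only when no minute carry occurs, it also sets the timer text blocks to near-white.
; The actor destroys itself after either branch.
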(event `self.Box.OnComponentBeginOverlap`
  (params (OverlappedComponent :type "PrimitiveComponent Object Reference") (OtherActor :type "Actor Object Reference") (OtherComp :type "PrimitiveComponent Object Reference") (OtherBodyIndex :type Integer) (bFromSweep :type Boolean) (SweepResult :type "HitResult Structure (by ref)"))
  (bind _ui_time_limit (`self.UI Time Limit`))
  (bind _ui_time_limit_2 (`self.UI Time Limit`))
  (bind _ui_time_limit_3 (`self.UI Time Limit`))
  (bind _second (`/Game/Takumi_Time_Battery/UI_TimeLimit.Second` (`self.UI Time Limit`)))
  (bind _astop_down_character (cast `/Game/TopDownBP/Blueprints/TopDownCharacter` OtherActor))
  (bind _output_get (set `self.UI Time Limit` (`/Game/TopDownBP/Blueprints/TopDownCharacter.UI_TimeLimit` _astop_down_character)))
  (`UserWidget.PlayAnimation` _output_get (`/Game/Takumi_Time_Battery/UI_TimeLimit.PlusTime` _output_get) 0.0 1 "Forward" 1.0 false)
  (if (>= _second 50)
    (set `/Game/Takumi_Time_Battery/UI_TimeLimit.Minute` (+ (`/Game/Takumi_Time_Battery/UI_TimeLimit.Minute` _ui_time_limit_2) 1) _ui_time_limit_2)
    (set `/Game/Takumi_Time_Battery/UI_TimeLimit.Second` (- 10 (- 60 (`/Game/Takumi_Time_Battery/UI_TimeLimit.Second` _ui_time_limit_3))) _ui_time_limit_3)
    (`/Game/Takumi_Time_Battery/UI_TimeLimit.SetString` (`self.UI Time Limit`))
    (`self.K2_DestroyActor`)
    (else
      (set `/Game/Takumi_Time_Battery/UI_TimeLimit.Second` (+ _second 10) (`self.UI Time Limit`))
      (`/Game/Takumi_Time_Battery/UI_TimeLimit.SetString` _ui_time_limit)
      (`TextBlock.SetColorAndOpacity` (`/Game/Takumi_Time_Battery/UI_TimeLimit.MinuteTextBlock` _ui_time_limit) (make `SlateColor` (struct :`R` 0.994792 :`G` 0.994792 :`B` 0.994792 :`A` 1.0)))
      (`TextBlock.SetColorAndOpacity` (`/Game/Takumi_Time_Battery/UI_TimeLimit.SecondTextBlock` _ui_time_limit) (make `SlateColor` (struct :`R` 0.994792 :`G` 0.994792 :`B` 0.994792 :`A` 1.0)))
      (`TextBlock.SetColorAndOpacity` (`/Game/Takumi_Time_Battery/UI_TimeLimit.TextBlock` _ui_time_limit) (make `SlateColor` (struct :`R` 0.994792 :`G` 0.994792 :`B` 0.994792 :`A` 1.0)))
      (`self.K2_DestroyActor`))))

(fn `UserConstructionScript`)