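; BP_Door is an automatic double door that opens when an actor tagged Player enters its Box trigger and closes when it leaves.
; BeginPlay stores each panel's closed relative location.
; A timeline, played or reversed on overlap, lerps both panels toward their open marker components in X and Y, keeping the closed Z.
; Door_Cue plays at the actor's location on both opening and closing.
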(event `self.ReceiveBeginPlay`
  (set `self.CloseLocation1` (`SceneComponent.RelativeLocation` (`self.1Door`)))
  (set `self.CloseLocation2` (`SceneComponent.RelativeLocation` (`self.2Door`))))

(event `self.Box.OnComponentBeginOverlap`
  (params (OverlappedComponent :type "PrimitiveComponent Object Reference") (OtherActor :type "Actor Object Reference") (OtherComp :type "PrimitiveComponent Object Reference") (OtherBodyIndex :type Integer) (bFromSweep :type Boolean) (SweepResult :type "HitResult Structure (by ref)"))
  (bind (_closelocation1_x _closelocation1_y _closelocation1_z) (`KismetMathLibrary.BreakVector` (`self.CloseLocation1`)))
  (bind (_closelocation2_x _closelocation2_y _closelocation2_z) (`KismetMathLibrary.BreakVector` (`self.CloseLocation2`)))
  (if (`self.ActorHasTag` OtherActor "Player")
    (`GameplayStatics.PlaySoundAtLocation` "/Game/HARUTO/SE/Door_Cue.Door_Cue" (`self.K2_GetActorLocation`) (struct) 1.0 1.0 0.0 null null null)
    (bind (_direction `_新規track_0`) (`Timeline|タイムライン_0` :!label _label)
      (:`Update`
        (bind (_returnvalue_x _returnvalue_y) (`KismetMathLibrary.BreakVector` (`KismetMathLibrary.VLerp` (`self.CloseLocation1`) (`SceneComponent.RelativeLocation` (`self.1_OpenLocation`)) `_新規track_0`)))
        (`SceneComponent.K2_SetRelativeLocation` (`self.1Door`) (`KismetMathLibrary.MakeVector` _returnvalue_x _returnvalue_y _closelocation1_z) false false)
        (bind (_returnvalue_x_2 _returnvalue_y_2) (`KismetMathLibrary.BreakVector` (`KismetMathLibrary.VLerp` (`self.CloseLocation2`) (`SceneComponent.RelativeLocation` (`self.2_OpenLocation`)) `_新規track_0`)))
        (`SceneComponent.K2_SetRelativeLocation` (`self.2Door`) (`KismetMathLibrary.MakeVector` _returnvalue_x_2 _returnvalue_y_2 _closelocation2_z) false false)))))

(event `self.Box.OnComponentEndOverlap`
  (params (OverlappedComponent :type "PrimitiveComponent Object Reference") (OtherActor :type "Actor Object Reference") (OtherComp :type "PrimitiveComponent Object Reference") (OtherBodyIndex :type Integer))
  (if (`self.ActorHasTag` OtherActor "Player")
    (`GameplayStatics.PlaySoundAtLocation` "/Game/HARUTO/SE/Door_Cue.Door_Cue" (`self.K2_GetActorLocation`) (struct) 1.0 1.0 0.0 null null null)
    (goto _label :!via `Reverse`)))

(fn `UserConstructionScript`)