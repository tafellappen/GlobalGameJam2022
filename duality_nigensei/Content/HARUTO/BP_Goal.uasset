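; BP_Goal is a level goal that ends the game and raises a lift platform when the player reaches it.
; A box overlap by a Player-tagged actor blends the camera to the goal and calls EndGame on the cached TopDownCharacter.
; After a short delay, a timeline lerps the platform from its current relative location toward the UpLocation component on each update.
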(event `self.ReceiveBeginPlay`
  (bind _astop_down_character (cast `/Game/TopDownBP/Blueprints/TopDownCharacter` (`GameplayStatics.GetPlayerPawn` 0)))
  (set `self.BP_Player` _astop_down_character))

(event `self.Box.OnComponentBeginOverlap`
  (params (OverlappedComponent :type "PrimitiveComponent Object Reference") (OtherActor :type "Actor Object Reference") (OtherComp :type "PrimitiveComponent Object Reference") (OtherBodyIndex :type Integer) (bFromSweep :type Boolean) (SweepResult :type "HitResult Structure (by ref)"))
  (bind _sm_lift_platform (`self.SM_Lift_Platform`))
  (if (`self.ActorHasTag` OtherActor "Player")
    (`PlayerController.SetViewTargetWithBlend` (`GameplayStatics.GetPlayerController` 0) self 2.0 "VTBlend_EaseOut" 0.5 false)
    ;[1 1 1] ここでプレイヤーの動きをなくす(Make the player inoperable here)
    (`/Game/TopDownBP/Blueprints/TopDownCharacter.EndGame` (`self.BP_Player`))
    (`KismetSystemLibrary.Delay` 2.5)
    (bind (_direction `_新規track_0`) (`Timeline|タイムライン_0` :!via `PlayFromStart`)
      (:`Update`
        (`SceneComponent.K2_SetRelativeLocation` _sm_lift_platform (`KismetMathLibrary.VLerp` (`SceneComponent.RelativeLocation` _sm_lift_platform) (`SceneComponent.RelativeLocation` (`self.UpLocation`)) `_新規track_0`) false false)))))

(fn `UserConstructionScript`)